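; A modular maze cell actor whose construction script builds a floor plus optional north, south, east and west walls and ceiling from scaled cube meshes.
; Grid size drives lengths and thickness, while wall height is set separately.
; Ceilinged cells with positive intensity get a centered point light colored at construction.
; Tick copies the third-person character's LightToChange into LightColor but does not update the existing light component.
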(event EventBeginPlay
  (bind _asbp_third_person_character (Utilities|Casting|CastToBP_ThirdPersonCharacter (Game|Player|GetPlayerPawn 0)))
  (Variables|Default|SetAs%20BP%20Third%20Person%20Character _asbp_third_person_character))

(event EventTick
  (params (DeltaSeconds :type Float%20%28single-precision%29))
  (Variables|Default|SetLightColor (Variables|/Game/ThirdPerson/Blueprints/BP_ThirdPersonCharacter.BP_ThirdPersonCharacter_C|Getlight%20to%20change (Variables|Default|GetAs%20BP%20Third%20Person%20Character))))

(fn ConstructionScript
  (bind _gridsize (Variables|Default|GetGridSize))
  (bind _gridsize_2 (Variables|Default|GetGridSize))
  (bind _returnvalue (* _gridsize_2 0.5))
  (LocalVariables|SetWallLength _gridsize)
  (LocalVariables|SetWallThickness (* _gridsize 0.1))
  (Transformation|SetRelativeScale3D (Variables|Default|GetFloor) (Utilities|SizetoCubeScale (Math|Vector|MakeVector (LocalVariables|GetWallLength) (LocalVariables|GetWallLength) (LocalVariables|GetWallThickness))))
  (if (Variables|Default|GetWestWall)
    (AddComponent|AddStaticMeshComponent false (Math|Transform|MakeTransform (Math|Vector|MakeVector 0.0 0.0 0.0) "0, 0, 0" (Utilities|SizetoCubeScale (Math|Vector|MakeVector (LocalVariables|GetWallLength) (LocalVariables|GetWallThickness) (Variables|Default|GetWallHeight))))))
  (if (Variables|Default|GetEastWall)
    (AddComponent|AddStaticMeshComponent false (Math|Transform|MakeTransform (Math|Vector|MakeVector 0.0 (- (LocalVariables|GetWallLength) (LocalVariables|GetWallThickness)) 0.0) "0, 0, 0" (Utilities|SizetoCubeScale (Math|Vector|MakeVector (LocalVariables|GetWallLength) (LocalVariables|GetWallThickness) (Variables|Default|GetWallHeight))))))
  (if (Variables|Default|GetSouthWall)
    (AddComponent|AddStaticMeshComponent false (Math|Transform|MakeTransform (Math|Vector|MakeVector 0.0 0.0 0.0) "0, 0, 0" (Utilities|SizetoCubeScale (Math|Vector|MakeVector (LocalVariables|GetWallThickness) (LocalVariables|GetWallLength) (Variables|Default|GetWallHeight))))))
  (if (Variables|Default|GetNorthWall)
    (AddComponent|AddStaticMeshComponent false (Math|Transform|MakeTransform (Math|Vector|MakeVector (- (LocalVariables|GetWallLength) (LocalVariables|GetWallThickness)) 0.0 0.0) "0, 0, 0" (Utilities|SizetoCubeScale (Math|Vector|MakeVector (LocalVariables|GetWallThickness) (LocalVariables|GetWallLength) (Variables|Default|GetWallHeight))))))
  (if (Variables|Default|GetCeiling)
    (AddComponent|AddStaticMeshComponent false (Math|Transform|MakeTransform (Math|Vector|MakeVector 0.0 0.0 (- (LocalVariables|GetWallLength) (LocalVariables|GetWallThickness))) "0, 0, 0" (Utilities|SizetoCubeScale (Math|Vector|MakeVector (LocalVariables|GetWallLength) (LocalVariables|GetWallLength) (LocalVariables|GetWallThickness)))))
    (if (Variables|Default|GetCeiling)
      (if (> (Variables|Default|GetLightIntensity) 0.0)
        (bind _returnvalue_2 (AddComponent|AddPointLightComponent false (Math|Transform|MakeTransform (Math|Vector|MakeVector _returnvalue _returnvalue (* (Variables|Default|GetWallHeight) 0.75)) "0, 0, 0" "1.000000,1.000000,1.000000")))
        (Rendering|Components|Light|SetLightColor _returnvalue_2 (Variables|Default|GetLightColor) true)
        (Rendering|Components|Light|SetIntensity _returnvalue_2 (Variables|Default|GetLightIntensity))))))